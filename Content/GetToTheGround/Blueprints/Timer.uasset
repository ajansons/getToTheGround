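; HUD Blueprint that draws a level timer, on-screen control instructions and a temporary "Level Complete!" banner.
; Tick counts down the clamped banner timer to toggle that message, and increments Time through a one-second Delay until EndofLevel is set.
; EndofLevel is only read here, and the debug prints of the three level times are unconnected.
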(event `self.ReceiveBeginPlay`)

(event `self.ReceiveActorBeginOverlap`
  (params (OtherActor :type "Actor Object Reference")))

(event `self.ReceiveDrawHUD`
  (params (SizeX :type Integer) (SizeY :type Integer))
  (`self.DrawText` (`KismetStringLibrary.Concat_StrStr` "Time: " (`KismetTextLibrary.Conv_TextToString` (`KismetTextLibrary.Conv_IntToText` (`KismetMathLibrary.FTrunc` (`self.Time`))))) (struct :`R` 1.0 :`B` 0.717532 :`A` 1.0) (* (`KismetMathLibrary.Conv_IntToDouble` SizeX) 0.85) (* (`KismetMathLibrary.Conv_IntToDouble` SizeY) 0.1) null 2.0)
  (`self.DrawText` "A and D to go left and right \nMouse to balance \nGet to the red box \nAvoid the sky!" (struct :`R` 0.963944 :`G` 1.0 :`B` 0.979755 :`A` 0.783) 30.0 30.0 null 2.0)
  (if (`self.DisplayNextLeveText`)
    (`self.DrawText` "Level Complete!" (struct :`R` 0.963944 :`G` 1.0 :`B` 0.979755 :`A` 0.783) (* SizeX 0.3) (* SizeY 0.3) null 5.0)))

(event `self.ReceiveTick`
  (params (DeltaSeconds :type "Float (single-precision)"))
  (bind _output_get (set `self.TimeToShowLevelText` (`KismetMathLibrary.FClamp` (- (`self.TimeToShowLevelText`) DeltaSeconds) 0.0 3.0)))
  (set `self.DisplayNextLeveText` (not (<= _output_get 0.0)))
  (if (not (`self.EndofLevel`))
    (`KismetSystemLibrary.Delay` 1.0)
    (set `self.Time` (+ (`self.Time`) 1.0))))

(fn `UserConstructionScript`)