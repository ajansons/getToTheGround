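; Junk is a physics-driven debris actor that takes a random variant each time it is constructed.
; The Construction Script switches on a random integer to add one of eleven static mesh components, with the default branch sharing case 0, so that variant is twice as likely.
; The added component simulates physics with gravity and receives a very large random torque around X.
; The Event Graph holds only disabled placeholder events.
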(event `self.ReceiveBeginPlay`)

(event `self.ReceiveActorBeginOverlap`
  (params (OtherActor :type "Actor Object Reference")))

(event `self.ReceiveTick`
  (params (DeltaSeconds :type "Float (single-precision)")))

(fn `UserConstructionScript`
  (bind _returnvalue (`KismetMathLibrary.MakeVector` (* (`KismetMathLibrary.RandomFloat`) 999999999.0)))
  (switch `int` (`KismetMathLibrary.RandomInteger` 12)
    (:`Default`
      (bind _returnvalue_2 (`AddComponent|Static Mesh Component_1017` :!label _label))
      (`PrimitiveComponent.SetSimulatePhysics` _returnvalue_2 true)
      (`PrimitiveComponent.SetEnableGravity` _returnvalue_2 true)
      (`PrimitiveComponent.AddTorque` _returnvalue_2 _returnvalue "None" false))
    (:`0`
      (goto _label))
    (:`1`
      (bind _returnvalue_3 (`AddComponent|StaticMeshComponent_827`))
      (`PrimitiveComponent.SetSimulatePhysics` _returnvalue_3 true)
      (`PrimitiveComponent.SetEnableGravity` _returnvalue_3 true)
      (`PrimitiveComponent.AddTorque` _returnvalue_3 _returnvalue "None" false))
    (:`2`
      (bind _returnvalue_4 (`AddComponent|StaticMeshComponent_832`))
      (`PrimitiveComponent.SetSimulatePhysics` _returnvalue_4 true)
      (`PrimitiveComponent.SetEnableGravity` _returnvalue_4 true)
      (`PrimitiveComponent.AddTorque` _returnvalue_4 _returnvalue "None" false))
    (:`3`
      (bind _returnvalue_5 (`AddComponent|StaticMeshComponent_4515`))
      (`PrimitiveComponent.SetSimulatePhysics` _returnvalue_5 true)
      (`PrimitiveComponent.SetEnableGravity` _returnvalue_5 true)
      (`PrimitiveComponent.AddTorque` _returnvalue_5 _returnvalue "None" false))
    (:`4`
      (bind _returnvalue_6 (`AddComponent|StaticMeshComponent_4516`))
      (`PrimitiveComponent.SetSimulatePhysics` _returnvalue_6 true)
      (`PrimitiveComponent.SetEnableGravity` _returnvalue_6 true)
      (`PrimitiveComponent.AddTorque` _returnvalue_6 _returnvalue "None" false))
    (:`5`
      (bind _returnvalue_7 (`AddComponent|StaticMeshComponent_4517`))
      (`PrimitiveComponent.SetSimulatePhysics` _returnvalue_7 true)
      (`PrimitiveComponent.SetEnableGravity` _returnvalue_7 true)
      (`PrimitiveComponent.AddTorque` _returnvalue_7 _returnvalue "None" false))
    (:`6`
      (bind _returnvalue_8 (`AddComponent|StaticMeshComponent_4518`))
      (`PrimitiveComponent.SetSimulatePhysics` _returnvalue_8 true)
      (`PrimitiveComponent.SetEnableGravity` _returnvalue_8 true)
      (`PrimitiveComponent.AddTorque` _returnvalue_8 _returnvalue "None" false))
    (:`7`
      (bind _returnvalue_9 (`AddComponent|StaticMeshComponent_4519`))
      (`PrimitiveComponent.SetSimulatePhysics` _returnvalue_9 true)
      (`PrimitiveComponent.SetEnableGravity` _returnvalue_9 true)
      (`PrimitiveComponent.AddTorque` _returnvalue_9 _returnvalue "None" false))
    (:`8`
      (bind _returnvalue_10 (`AddComponent|StaticMeshComponent_49`))
      (`PrimitiveComponent.SetSimulatePhysics` _returnvalue_10 true)
      (`PrimitiveComponent.SetEnableGravity` _returnvalue_10 true)
      (`PrimitiveComponent.AddTorque` _returnvalue_10 _returnvalue "None" false))
    (:`9`
      (bind _returnvalue_11 (`AddComponent|StaticMeshComponent_50`))
      (`PrimitiveComponent.SetSimulatePhysics` _returnvalue_11 true)
      (`PrimitiveComponent.SetEnableGravity` _returnvalue_11 true)
      (`PrimitiveComponent.AddTorque` _returnvalue_11 _returnvalue "None" false))
    (:`10`
      (bind _returnvalue_12 (`AddComponent|StaticMeshComponent_51`))
      (`PrimitiveComponent.SetSimulatePhysics` _returnvalue_12 true)
      (`PrimitiveComponent.SetEnableGravity` _returnvalue_12 true)
      (`PrimitiveComponent.AddTorque` _returnvalue_12 _returnvalue "None" false))))