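; House actor Blueprint that can return its house mesh to where it started.
; BeginPlay caches the HouseMesh world location and rotation.
; The ResetPosition function restores both values without sweep or teleport, so other logic can put the house back after it moves.
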(event `self.ReceiveBeginPlay`
  (bind _housemesh (`self.HouseMesh`))
  (set `self.StartingTransform` (`SceneComponent.K2_GetComponentLocation` _housemesh))
  (set `self.StartingRotation` (`SceneComponent.K2_GetComponentRotation` _housemesh)))

(event `self.ReceiveActorBeginOverlap`
  (params (OtherActor :type "Actor Object Reference")))

(event `self.ReceiveTick`
  (params (DeltaSeconds :type "Float (single-precision)")))

(fn `ResetPosition`
  (bind _housemesh (`self.HouseMesh`))
  (`SceneComponent.K2_SetWorldLocation` _housemesh (`self.StartingTransform`) false false)
  (`SceneComponent.K2_SetWorldRotation` _housemesh (`self.StartingRotation`) false false))

(fn `UserConstructionScript`)